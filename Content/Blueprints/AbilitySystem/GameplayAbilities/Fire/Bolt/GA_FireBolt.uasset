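; GA_FireBolt is a gameplay ability that fires a fire bolt projectile toward the point under the mouse cursor.
; Activation gets target data under the mouse, turns the avatar toward the hit location through CombatInterface and plays the bolt cast montage.
; A montage gameplay event triggers the projectile spawn at that target, then the ability ends after a short delay.
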(event `self.K2_ActivateAbility`
  (bind (_asynctaskproxy _datahandle) (`TargetDataUnderMouse.CreateTargetDataUnderMouse`)
    (:`ValidData`
      (set `self.TargetLocation` (`.Location` (`GameplayStatics.BreakHitResult` (`AbilitySystemBlueprintLibrary.GetHitResultFromTargetData` _datahandle))))
      (bind _ascombat_interface (cast `CombatInterface` (`self.GetAvatarActorFromActorInfo`)))
      (`CombatInterface.SetFacingTarget` _ascombat_interface (`self.TargetLocation`))
      (`AbilityTask_PlayMontageAndWait.CreatePlayMontageAndWaitProxy` "None" "/Game/Assets/Characters/Aura/Animations/Abilities/AM_CastBolt.AM_CastBolt"
        (:`then`
          (`AbilityTask_WaitGameplayEvent.WaitGameplayEvent` (struct :`TagName` "Event.Montage.Bolt") null
            (:`EventReceived`
              (`self.SpawnProjectile` (`self.TargetLocation`))
              (`KismetSystemLibrary.Delay` 0.6)
              (`self.K2_EndAbility`))))))))